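; Spike trap actor that continuously fires SpikeProjectile actors from five socket components, one socket at a time.
; BeginPlay collects the sockets into an array, and Tick accumulates a timer that triggers shots at a ShotsPerSecond rate.
; Each shot spawns a projectile at the current socket's transform with a debug sphere, then advances the index with modulo wraparound.
; An unused line-trace prototype for instant-hit shots remains disconnected.
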(event EventBeginPlay
  ;[0.06271 0.03913 0.1615] well... Add sockets... for arrows...
  (Utilities|Array|Add (Variables|Default|GetSocketArray) (Variables|Default|GetFireSocket))
  (Utilities|Array|Add (Variables|Default|GetSocketArray) (Variables|Default|GetFireSocket1))
  (Utilities|Array|Add (Variables|Default|GetSocketArray) (Variables|Default|GetFireSocket2))
  (Utilities|Array|Add (Variables|Default|GetSocketArray) (Variables|Default|GetFireSocket3))
  (Utilities|Array|Add (Variables|Default|GetSocketArray) (Variables|Default|GetFireSocket4)))

(event Collision|EventActorBeginOverlap
  (params (OtherActor :type Actor%20Object%20Reference)))

(event EventTick
  (params (DeltaSeconds :type Float%20%28single-precision%29))
  (bind _shotspersecond (Variables|Default|GetShotsPerSecond))
  (bind _returnvalue (/ 1.0 _shotspersecond))
  ;[0.7643 1 0.669] Timer stuff
  ;;[1 1 1] Increment shot timer
  (bind _output_get (Variables|Default|SetshotTimer (+ DeltaSeconds (Variables|Default|GetshotTimer))))
  ;;[1 1 1] Check if shot is ready
  (if (> _output_get _returnvalue)
    ;;[1 1 1] decrement shot timer
    (Variables|Default|SetshotTimer (- (Variables|Default|GetshotTimer) _returnvalue))
    ;[0.3906 0.2123 0.1333] Cycle Sockets
    (for (_ _array_index) (Variables|Default|GetSocketArray)
      (if (== _array_index (Variables|Default|GetArrow%20socket%20iterator))
        ;[1 1 1] Check if sockets cycle properly
        (Rendering|Debug|DrawDebugSphere (.location (Transformation|GetWorldTransform (Utilities|Array|Get(acopy) (Variables|Default|GetSocketArray) _array_index))) 3e+01 12 "(R=1.000000,G=1.000000,B=1.000000,A=1.000000)" (/ 1.0 (Variables|Default|GetShotsPerSecond)))
        (Game|SpawnActorfromClass "/Game/Blueprints/SpikeTrap/SpikeProjectile.SpikeProjectile_C" (Transformation|GetWorldTransform (Utilities|Array|Get(acopy) (Variables|Default|GetSocketArray) _array_index)) "Undefined" "MultiplyWithRoot" 0 0)))
    (Variables|Default|SetArrow%20socket%20iterator (Math|Integer|%(Integer) (+ (Variables|Default|GetArrow%20socket%20iterator) 1) (Utilities|Array|Length (Variables|Default|GetSocketArray))))))

(fn ConstructionScript)