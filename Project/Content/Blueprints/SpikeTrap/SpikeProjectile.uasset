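; SpikeProjectile is a spike trap projectile that restarts the current level when something overlaps it.
; An overlap on its Sphere1 component reopens the current level by name, with no check on the overlapping actor.
; Tick accumulates a lifetime counter and destroys the actor once it exceeds a maximum, so stray projectiles do not persist.
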(event OnComponentBeginOverlap(Sphere1)
  (params (OverlappedComponent :type Primitive%20Component%20Object%20Reference) (OtherActor :type Actor%20Object%20Reference) (OtherComp :type Primitive%20Component%20Object%20Reference) (OtherBodyIndex :type Integer) (bFromSweep :type Boolean) (SweepResult :type Hit%20Result%20Structure%20%28by%20ref%29))
  ;[1 1 1] Reset current level
  (bind _returnvalue (Game|GetCurrentLevelName true))
  (Game|OpenLevel(byName) (Utilities|String|StringToName _returnvalue)))

(event EventBeginPlay)

(event Collision|EventActorBeginOverlap
  (params (OtherActor :type Actor%20Object%20Reference)))

(event EventTick
  (params (DeltaSeconds :type Float%20%28single-precision%29))
  (Utilities|FlowControl|Sequence
    (:then_0
      ;[1 1 1] Despawn after X time to not have infinite
      (if (> (Variables|Default|GetLifetimeCurr) (Variables|Default|GetLifeTimeMax))
        (Actor|DestroyActor)))
    (:then_1
      ;[1 1 1] Check DespawnTimer
      (Variables|Default|SetLifetimeCurr (+ DeltaSeconds (Variables|Default|GetLifetimeCurr))))))

(fn ConstructionScript)