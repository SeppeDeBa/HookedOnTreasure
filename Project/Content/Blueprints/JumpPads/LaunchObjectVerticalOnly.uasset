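; Jump pad Blueprint that bounces the player character vertically, like a trampoline.
; On Box overlap, a falling BP_PlayerCharacter is launched with its Z velocity inverted, overriding only the vertical axis so horizontal movement carries through.
; Rising or level characters are unaffected, and other actors only print a cast failure.
; An alternative launch along the pad's up vector using LaunchStrength is left disconnected.
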(event OnComponentBeginOverlap(Box)
  (params (OverlappedComponent :type Primitive%20Component%20Object%20Reference) (OtherActor :type Actor%20Object%20Reference) (OtherComp :type Primitive%20Component%20Object%20Reference) (OtherBodyIndex :type Integer) (bFromSweep :type Boolean) (SweepResult :type Hit%20Result%20Structure%20%28by%20ref%29))
  (bind _asbp_player_character (Utilities|Casting|CastToBP_PlayerCharacter OtherActor)
    (:then
      ;[1 1 1] if velocity is negative
      (if (< (.z (Variables|/Script/Engine.MovementComponent|GetVelocity (Variables|/Script/Engine.Character|GetCharacterMovement _asbp_player_character))) 0.0)
        (Character|LaunchCharacter _asbp_player_character (Math|Vector|MakeVector 0.0 0.0 (* (.z (Variables|/Script/Engine.MovementComponent|GetVelocity (Variables|/Script/Engine.Character|GetCharacterMovement _asbp_player_character))) -1.0)) false true)))
    (:CastFailed
      (Development|PrintString "cast failed"))))

(event EventBeginPlay)

(event Collision|EventActorBeginOverlap
  (params (OtherActor :type Actor%20Object%20Reference)))

(event EventTick
  (params (DeltaSeconds :type Float%20%28single-precision%29)))

(fn ConstructionScript)