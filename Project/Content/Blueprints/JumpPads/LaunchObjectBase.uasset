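; LaunchObjectBase is a jump pad actor, apparently a base for launch objects, that flings the player character when stepped into.
; Its Box overlap event casts to BP_PlayerCharacter and calls LaunchCharacter along the root component's up vector scaled by LaunchStrength, overriding existing velocity.
; Rotating the actor therefore aims the launch, and a 2D sound plays on each launch.
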(event OnComponentBeginOverlap(Box)
  (params (OverlappedComponent :type Primitive%20Component%20Object%20Reference) (OtherActor :type Actor%20Object%20Reference) (OtherComp :type Primitive%20Component%20Object%20Reference) (OtherBodyIndex :type Integer) (bFromSweep :type Boolean) (SweepResult :type Hit%20Result%20Structure%20%28by%20ref%29))
  (bind _asbp_player_character (Utilities|Casting|CastToBP_PlayerCharacter OtherActor))
  ;[1 1 1] Pieuw
  (Character|LaunchCharacter _asbp_player_character (* (Math|Vector|GetUpVector (Transformation|GetWorldRotation (Variables|Default|GetDefaultSceneRoot))) (Variables|Default|GetLaunch%20Strength)) true true)
  (Audio|PlaySound2D "/Engine/VREditor/Sounds/VR_ungrab.VR_ungrab" 1.0 1.0 0.0 0 0))

(event EventBeginPlay)

(event Collision|EventActorBeginOverlap
  (params (OtherActor :type Actor%20Object%20Reference)))

(event EventTick
  (params (DeltaSeconds :type Float%20%28single-precision%29)))

(fn ConstructionScript)