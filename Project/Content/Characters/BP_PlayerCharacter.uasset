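; Player character Blueprint with three movement abilities: skiing, grappling hook and airblast, plus visual feedback for each.
; Skiing zeroes ground friction, while grappling line-traces from the camera direction, switches to Flying, then pulls toward the hit each Tick with sideways steering.
; Airblast launches the character opposite the view, with a timed cooldown shown by a scaling gun bar.
; Tick also colors the HUD reticle by grapple range and updates the jump bracelet.
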(event Input|EnhancedActionEvents|EnhancedInputActionIA_Ski
  (params (ActionValue :type Boolean) (ElapsedSeconds :type Float%20%28double-precision%29) (TriggeredSeconds :type Float%20%28double-precision%29) (InputAction :type Input%20Action%20Object%20Reference :default "/Game/Input/Actions/IA_Ski.IA_Ski"))
  (bind _skibracelet (Variables|Default|GetSkiBracelet))
  ;[1 0 0] MainChar Specific Ability
  (:Started
    ;;[1 1 1] Start Skiing
    (Variables|/Script/Engine.CharacterMovementComponent|SetGroundFriction (Variables|Character|GetCharacterMovement) 0.0)
    (Development|PrintString "gliding activated")
    (Variables|Default|SetIsSkiing true)
    ;;[1 1 1] Visual update for player feedback
    (Rendering|Material|SetMaterial _skibracelet 0 "/Engine/VREditor/UI/ArrowMaterial.ArrowMaterial"))
  (:Completed
    ;;[1 1 1] Stop Skiing
    (Variables|/Script/Engine.CharacterMovementComponent|SetGroundFriction (Variables|Character|GetCharacterMovement) (Variables|Default|GetBaseFriction))
    (Development|PrintString "gliding deactivated")
    (Variables|Default|SetIsSkiing false)
    (Rendering|Material|SetMaterial _skibracelet 0 "/Engine/TemplateResources/MI_Template_BaseGray.MI_Template_BaseGray")))

(event Input|EnhancedActionEvents|EnhancedInputActionIA_AirBlast
  (params (ActionValue :type Boolean) (ElapsedSeconds :type Float%20%28double-precision%29) (TriggeredSeconds :type Float%20%28double-precision%29) (InputAction :type Input%20Action%20Object%20Reference :default "/Game/Input/Actions/IA_AirBlast.IA_AirBlast"))
  ;[1 0 0] MainChar only ability
  (:Triggered
    (if (Variables|AirblastGun|GetCanAirblast)
      ;;[1 1 1] Shoot character and set bool for visual updates
      (Character|LaunchCharacter (* (* (Transformation|GetActorForwardVector (Game|GetPlayerCameraManager 0)) -1) (Variables|AirblastGun|GetAirblastStrength)) false false)
      (Variables|AirblastGun|SetCanAirblast false)
      (Rendering|Material|SetMaterial (Variables|Components|GetAirblastCDBar) 0 "/Engine/VREditor/LaserPointer/LaserPointerMaterialInst.LaserPointerMaterialInst")
      (Components|Activation|Activate (Variables|Components|GetFX_AirBlast) true)
      (Audio|PlaySound2D "/Game/StarterContent/Audio/Explosion02.Explosion02" 1.0 1.0 0.0 0 0))))

(event Input|EnhancedActionEvents|EnhancedInputActionIA_Grapple
  (params (ActionValue :type Boolean) (ElapsedSeconds :type Float%20%28double-precision%29) (TriggeredSeconds :type Float%20%28double-precision%29) (InputAction :type Input%20Action%20Object%20Reference :default "/Game/Input/Actions/IA_Grapple.IA_Grapple"))
  (bind _sphere (Variables|Components|GetSphere))
  (bind _returnvalue (Transformation|GetWorldLocation _sphere))
  ;[1 0 0] Th Grappling hook beast
  (:Triggered
    (if (not (Variables|BasicGrappling|GetIsSwinging))
      ;;[1 1 1] RayTrace
      (bind (_outhit _returnvalue_2) (Collision|LineTraceByChannel _returnvalue (+ _returnvalue (* (Variables|BasicGrappling|GetGrappling_Range) (Math|Vector|GetForwardVector (Transformation|GetWorldRotation (Variables|Components|GetCameraComponent))))) "TraceTypeQuery1" false 0 "None" true "(R=1.000000,G=0.000000,B=0.000000,A=1.000000)" "(R=0.000000,G=1.000000,B=0.000000,A=1.000000)" 2.0))
      (if _returnvalue_2
        ;;[1 1 1] Save grapple point and set grappling state (for now bool)
        (Variables|BasicGrappling|SetGrapplingPoint (.ImpactPoint (Collision|BreakHitResult _outhit)))
        (Variables|BasicGrappling|SetIsSwinging true)
        ;;[1 1 1] Could maybe be custom movement mode?
        (Pawn|Components|CharacterMovement|SetMovementMode (Variables|Character|GetCharacterMovement) "MOVE_Flying" 0)
        ;;[1 1 1] Show cable
        (Rendering|SetVisibility (Variables|Components|GetGrappling%20rope) true false)
        (Audio|PlaySound2D "/Engine/VREditor/Sounds/UI/Gizmo_Handle_Clicked.Gizmo_Handle_Clicked" 1.0 1.0 0.0 0 0))))
  (:Completed
    ;;[1 1 1] Hide grapple and set state
    (Rendering|SetVisibility (Variables|Components|GetGrappling%20rope) false false)
    (Variables|BasicGrappling|SetIsSwinging false)
    ;;[1 1 1] If not grappling, set to falling
    (Pawn|Components|CharacterMovement|SetMovementMode (Variables|Character|GetCharacterMovement) "MOVE_Falling" 0)))

(event Collision|EventActorBeginOverlap
  (params (OtherActor :type Actor%20Object%20Reference)))

(event EventTick
  (params (DeltaSeconds :type Float%20%28single-precision%29))
  (bind _airblastcdbar (Variables|Components|GetAirblastCDBar))
  (bind _sphere (Variables|Components|GetSphere))
  (bind _returnvalue (Transformation|GetWorldLocation _sphere))
  (bind _relativescale3d (Variables|/Script/Engine.SceneComponent|GetRelativeScale3D _airblastcdbar))
  (Utilities|FlowControl|Sequence
    (:then_0
      ;[1 0.6527 0.1765] 1. Grappling pull in physics
      (if (Variables|BasicGrappling|GetIsSwinging)
        ;;[1 1 1] Save End Location for movement usage
        (Variables|/Script/CableComponent.CableComponent|SetEndLocation (Variables|Components|GetGrappling%20rope) (Math|Transform|InverseTransformLocation (Transformation|GetActorTransform) (Variables|BasicGrappling|GetGrapplingPoint)))
        (Physics|AddForce (Variables|Character|GetCharacterMovement) (* (Math|Vector|Normalize (+ (Math|Vector|GetUnitDirection(Vector) (Transformation|GetActorLocation) (Variables|BasicGrappling|GetGrapplingPoint)) (* (* (Transformation|GetActorRightVector) (.x (Input|EnhancedActionValues|GetIA_PlayerMovement))) (Variables|BasicGrappling|GetSidewaysInputInfluenceFactor)))) (Variables|BasicGrappling|GetGrapplingStrength)))))
    (:then_1
      ;[1 0.739 0.2663] 2. Airblast
      (if (not (Variables|AirblastGun|GetCanAirblast))
        (Variables|AirblastGun|SetAirBlastTimer (+ (Variables|AirblastGun|GetAirBlastTimer) DeltaSeconds))
        (Transformation|SetRelativeScale3D _airblastcdbar (Math|Vector|MakeVector (* (/ (Variables|AirblastGun|GetAirBlastTimer) (Variables|AirblastGun|GetAirBlastCD)) (Variables|AirblastGun|GetGunAirblastTargetScale)) (.y _relativescale3d) (.z _relativescale3d)))
        (if (> (Variables|AirblastGun|GetAirBlastTimer) (Variables|AirblastGun|GetAirBlastCD))
          (Variables|AirblastGun|SetCanAirblast true)
          (Rendering|Material|SetMaterial (Variables|Components|GetAirblastCDBar) 0 "/Engine/VREditor/UI/FrameMaterial.FrameMaterial")
          (Variables|AirblastGun|SetAirBlastTimer 0.0))))
    (:then_2
      ;[1 0.7041 0.2686] 3. PlayerFeedback range indicator crosshair
      ;;[1 1 1] RayTrace
      (bind _returnvalue_2 (Collision|LineTraceByChannel _returnvalue (+ _returnvalue (* (Variables|BasicGrappling|GetGrappling_Range) (Math|Vector|GetForwardVector (Transformation|GetWorldRotation (Variables|Components|GetCameraComponent))))) "TraceTypeQuery1" false 0 "None" true "(R=1.000000,G=0.000000,B=0.000000,A=1.000000)" "(R=0.000000,G=1.000000,B=0.000000,A=1.000000)" 2.0))
      ;;[1 1 1] Update center of screen aiming reticle if in range
      (Default|CheckandSetReticleColor (Variables|Default|GetUI_HUD%20Class%20Ref) _returnvalue_2))
    (:then_3
      ;[0.6793 1 0.6457] 4. Air Jump bracelet Player Feedback Visual Update
      (Variables|Default|SetJumpAvailable (Character|CanJump))
      (if (Variables|Default|GetJumpAvailable)
        ;;[1 1 1] PlayerFeedback Visual Update
        (Rendering|Material|SetMaterial (Variables|Default|GetJumpBracelet) 0 "/Niagara/DefaultAssets/GeometryCache/M_DefaultGeometryCacheMaterial_Blue.M_DefaultGeometryCacheMaterial_Blue")
        (else
          (Rendering|Material|SetMaterial (Variables|Default|GetJumpBracelet) 0 "/Engine/TemplateResources/MI_Template_BaseGray.MI_Template_BaseGray"))))))

(event EventBeginPlay
  (Utilities|FlowControl|Sequence
    (:then_0
      ;[0 0.008147 0.2292] Future Seppe Here, Should have made a C++ custom HUD and managed it in there...
      ;;[0.2138 0.2401 1] Create Timer Widget, can be moved to a custom HUD, keeping for easy reference
      (bind _returnvalue (UserInterface|CreateWidget "/Game/UI/UI_HUD.UI_HUD_C"))
      (UserInterface|Viewport|AddtoViewport _returnvalue 0)
      (Variables|Default|SetUI_HUD%20Class%20Ref _returnvalue))
    (:then_1
      ;[1 1 1] Save target scale, gives freedom to replace and rescale the bar
      (Variables|AirblastGun|SetGunAirblastTargetScale (.x (Variables|/Script/Engine.SceneComponent|GetRelativeScale3D (Variables|Components|GetAirblastCDBar)))))))

(fn ConstructionScript
  (|CallParentFunction))